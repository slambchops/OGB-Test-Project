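; Player character that layers equipment, item use and death handling onto inherited locomotion with mantle, roll, sprint and ragdoll.
; Separate graphs route movement input to locomotion and action input to OGBEquipment's active item.
; Equipment changes drive the animation overlay, while certain locomotion starts drop carried items or holster.
; OGBHealth triggers ragdoll at zero health; the authority also notifies the controller and detaches the pawn; K applies self-damage.
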(event EventBeginPlay
  ;[1 1 1] Bind health events
  (EventDispatchers|BindEventtoOnHealthChanged (Variables|Default|GetOGBHealth) (EventDispatchers|CreateEvent :!event OnHealthChanged))
  (Networking|SwitchHasAuthority
    (:Authority
      (EventDispatchers|BindEventtoOnTakeDamage (Variables|Default|GetOGBHealth) (EventDispatchers|CreateEvent :!event OnTakeDamage)))))

(event Collision|EventActorBeginOverlap
  (params (OtherActor :type Actor%20Object%20Reference)))

(event EventTick
  (params (DeltaSeconds :type Float%20%28single-precision%29)))

(event Input|KeyboardEvents|K
  (params (Key :type Key%20Structure))
  (:Pressed
    (Game|Damage|ApplyDamage self 1e+02 0 0)))

(event EventHandleMantleStart
  (params (MantleType :type EMantleType%20Enum :default "LowMantle"))
  ;[1 1 1] Locomotion state change events
  (|CallParentFunction MantleType)
  (switch Utilities|FlowControl|Switch|SwitchonEMantleType MantleType
    (:HighMantle
      _)
    (:FallingCatch
      _))
  (Class|OGBEquipmentComponent|SetActiveSlot (Variables|Default|GetOGBEquipment) "None")
  (Class|OGBEquipmentComponent|DropCarriedItem (Variables|Default|GetOGBEquipment)))

(event EventHandleRagdollStart
  ;[1 1 1] Locomotion state change events
  (|CallParentFunction)
  (Class|OGBEquipmentComponent|SetActiveSlot (Variables|Default|GetOGBEquipment) "None")
  (Class|OGBEquipmentComponent|DropCarriedItem (Variables|Default|GetOGBEquipment)))

(event EventHandleRollStart
  ;[1 1 1] Locomotion state change events
  (|CallParentFunction)
  (Class|OGBEquipmentComponent|DropCarriedItem (Variables|Default|GetOGBEquipment)))

(event EventHandleSprintStart
  ;[1 1 1] Locomotion state change events
  (|CallParentFunction)
  (Class|OGBEquipmentComponent|DropCarriedItem (Variables|Default|GetOGBEquipment)))

(event Input|AxisEvents|InputAxisMoveForward
  (params (AxisValue :type Float%20%28single-precision%29))
  ;[1 1 1] Input movement axis
  (Class|LocomotionCharacter|MoveForward AxisValue))

(event Input|AxisEvents|InputAxisMoveRight
  (params (AxisValue :type Float%20%28single-precision%29))
  ;[1 1 1] Input movement axis
  (Class|LocomotionCharacter|MoveRight AxisValue))

(event Input|AxisEvents|InputAxisLookUp
  (params (AxisValue :type Float%20%28single-precision%29))
  ;[1 1 1] Input movement axis
  (Pawn|Input|AddControllerPitchInput AxisValue))

(event Input|AxisEvents|InputAxisTurn
  (params (AxisValue :type Float%20%28single-precision%29))
  ;[1 1 1] Input movement axis
  (Pawn|Input|AddControllerYawInput AxisValue))

(event Input|MouseEvents|RightMouseButton
  (params (Key :type Key%20Structure))
  ;[1 1 1] Input Actions
  (:Pressed
    (Class|LocomotionCharacter|SetRotationMode "Aiming")))

(event Input|KeyboardEvents|LeftCtrl
  (params (Key :type Key%20Structure))
  ;[1 1 1] Input Actions
  (:Pressed
    (Class|LocomotionCharacter|BeginCrouch))
  (:Released
    (Class|LocomotionCharacter|EndCrouch)))

(event Input|KeyboardEvents|LeftShift
  (params (Key :type Key%20Structure))
  ;[1 1 1] Input Actions
  (:Pressed
    (Class|LocomotionCharacter|BeginSprint))
  (:Released
    (Class|LocomotionCharacter|EndSprint)))

(event Input|KeyboardEvents|LeftAlt
  (params (Key :type Key%20Structure))
  ;[1 1 1] Input Actions
  (:Pressed
    (Class|LocomotionCharacter|Roll)))

(event Input|KeyboardEvents|SpaceBar
  (params (Key :type Key%20Structure))
  ;[1 1 1] Input Actions
  (:Pressed
    (Character|Jump)))

(event Input|MouseEvents|LeftMouseButton
  (params (Key :type Key%20Structure))
  ;[1 1 1] Input Actions
  (:Pressed
    (Class|LocomotionCharacter|SetRotationMode "Aiming")))

(event Input|ActionEvents|InputActionInteract
  (params (Key :type Key%20Structure))
  ;[1 1 1] Item usage
  (:Pressed
    (Class|OGBInteractableInterface|BeginInteract(Message) (Variables|Default|GetInReachActor) self)))

(event Input|ActionEvents|InputActionDropCarriedItem
  (params (Key :type Key%20Structure))
  ;[1 1 1] Item usage
  (:Pressed
    (Class|OGBEquipmentComponent|DropCarriedItem (Variables|Default|GetOGBEquipment))))

(event Input|ActionEvents|InputActionPrimaryAction
  (params (Key :type Key%20Structure))
  ;[1 1 1] Item usage
  (:Pressed
    (ItemUsage|StartPrimaryAction))
  (:Released
    (ItemUsage|StopPrimaryAction)))

(event Input|ActionEvents|InputActionSelectFirstItem
  (params (Key :type Key%20Structure))
  ;[1 1 1] Item usage
  (:Pressed
    (bind _bcanuse (ItemUsage|CanUseItems))
    (if _bcanuse
      (Class|OGBEquipmentComponent|SetActiveSlot (Variables|Default|GetOGBEquipment) "Primary"))))

(event Input|ActionEvents|InputActionSelectSecondItem
  (params (Key :type Key%20Structure))
  ;[1 1 1] Item usage
  (:Pressed
    (bind _bcanuse (ItemUsage|CanUseItems))
    (if _bcanuse
      (Class|OGBEquipmentComponent|SetActiveSlot (Variables|Default|GetOGBEquipment) "Secondary"))))

(event Input|ActionEvents|InputActionReloadAction
  (params (Key :type Key%20Structure))
  ;[1 1 1] Item usage
  (:Pressed
    (bind _bcanuse (ItemUsage|CanUseItems))
    (if _bcanuse
      (ItemUsage|ReloadAction))))

(fn ConstructionScript)

(fn CanUseItems
  (bind _returnvalue (Class|LocomotionCharacter|IsDoingAction))
  (return (not _returnvalue)))

(fn StartPrimaryAction
  (ItemUsage|CanUseItems)
  (bind _returnvalue (Class|OGBEquipmentComponent|GetActiveItem (Variables|Default|GetOGBEquipment)))
  (Utilities|IsValid _returnvalue
    (:Is%20Valid
      (Class|OGBItemBase|PrimaryActionStart _returnvalue)
      (Class|LocomotionCharacter|SetRotationMode "Aiming")
      (Variables|Default|SetbLockAimingRotationMode true))))

(fn StopPrimaryAction
  (bind _returnvalue (Class|OGBEquipmentComponent|GetActiveItem (Variables|Default|GetOGBEquipment)))
  (Utilities|IsValid _returnvalue
    (:Is%20Valid
      (Class|OGBItemBase|PrimaryActionStop _returnvalue)
      (Variables|Default|SetbLockAimingRotationMode false))))

(fn ReloadAction
  (bind _bcanuse (ItemUsage|CanUseItems))
  (if _bcanuse
    (bind _returnvalue (Class|OGBEquipmentComponent|GetActiveItem (Variables|Default|GetOGBEquipment)))
    (Utilities|IsValid _returnvalue
      (:Is%20Valid
        (Class|OGBItemBase|ReloadActionStart _returnvalue)))))

(fn HandleAnimNotify
  (params (AnimNotify :type ELocoAnimNotify%20Enum :default "Equip"))
  (bind _returnvalue (Class|OGBEquipmentComponent|GetActiveItem (Variables|Default|GetOGBEquipment)))
  (Utilities|IsValid _returnvalue
    (:Is%20Valid
      (Class|OGBItemBase|HandleEquipAnimNotify _returnvalue)
      (return true))))

(fn HandleActiveEquipmentUpdate
  (params (Slot :type EEquipmentSlot%20Enum :default "None") (Item :type OGB%20Item%20Base%20Object%20Reference) (bNew :type Boolean))
  (Utilities|FlowControl|Sequence
    (:then_0
      ;[1 1 1] Set animation enum
      (Utilities|IsValid Item
        (:Is%20Valid
          (bind _returnvalue (Class|OGBItemBase|IsActive Item))
          (if _returnvalue
            (LocalVariables|SetNewAnim (Utilities|Enum|ByteToEnumEOverlayState (Variables|/Script/OGB_Gameplay_Core.OGBItemBase|GetAnimationEnum Item)))))))
    (:then_1
      ;[1 1 1] Update animation overlay
      (Class|LocomotionCharacter|SetOverlayState (LocalVariables|GetNewAnim)))))

(fn OnTakeDamage
  (params (HealthComp :type OGB%20Health%20Component%20Object%20Reference) (Health :type Float%20%28single-precision%29) (HealthDelta :type Float%20%28single-precision%29) (DamageType :type Damage%20Type%20Object%20Reference) (InstigatedBy :type Controller%20Object%20Reference) (DamageCauser :type Actor%20Object%20Reference))
  (if (<= Health 0.0)
    (Utilities|FlowControl|Sequence
      (:then_0
        (bind _asogbplayer_controller (Utilities|Casting|CastToOGBPlayerController (Pawn|GetController)))
        (Class|OGBPlayerController|OnPlayerKilled _asogbplayer_controller))
      (:then_1
        (Class|Pawn|DetachfromControllerPendingDestroy)
        (Actor|SetLifeSpan 1e+01)))))

(fn OnHealthChanged
  (params (Health :type Float%20%28single-precision%29))
  (if (<= Health 0.0)
    (Class|LocomotionCharacter|EnableRagdoll true)))

(fn OnCarriedItemChanged
  (params (Item :type OGB%20Item%20Base%20Object%20Reference))
  (Utilities|IsValid Item
    (:Is%20Valid
      (Class|LocomotionCharacter|SetOverlayState (Utilities|Enum|ByteToEnumEOverlayState (Variables|/Script/OGB_Gameplay_Core.OGBItemBase|GetAnimationEnum Item))))
    (:Is%20Not%20Valid
      (Class|LocomotionCharacter|SetOverlayState "Default")))
  (return true))

(fn OnEquipmentSlotChanged
  (params (Slot :type EEquipmentSlot%20Enum :default "None") (Item :type OGB%20Item%20Base%20Object%20Reference) (bActiveSlot :type Boolean) (bNewItem :type Boolean))
  (if bActiveSlot
    (CallFunction|HandleActiveEquipmentUpdate Slot Item bNewItem)
    (return true)))