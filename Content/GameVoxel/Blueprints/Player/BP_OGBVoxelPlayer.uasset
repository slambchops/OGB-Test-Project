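; BP_OGBVoxelPlayer is a player Blueprint that customizes how the player sets its movement base on voxel terrain.
; SetBase_BP detects voxel procedural mesh or instanced static mesh components owned by a VoxelWorld and passes that world's root component to SetBaseNative instead.
; It returns true for those cases and false otherwise, leaving other bases to default handling.
; The event graph and construction script add no logic of their own.
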(event EventBeginPlay
  (|CallParentFunction) ; This node is disabled and will not be called.\nDrag off pins to build functionality.
)

(event Collision|EventActorBeginOverlap
  (params (OtherActor :type Actor%20Object%20Reference))
  (|CallParentFunction OtherActor) ; This node is disabled and will not be called.\nDrag off pins to build functionality.
)

(event EventTick
  (params (DeltaSeconds :type Float%20%28single-precision%29))
  (|CallParentFunction DeltaSeconds) ; This node is disabled and will not be called.\nDrag off pins to build functionality.
)

(fn ConstructionScript
  (|CallParentFunction))

(fn SetBaseBP
  (params (NewBase :type Primitive%20Component%20Object%20Reference) (BoneName :type Name :default "None") (bNotifyActor :type Boolean))
  (Utilities|FlowControl|Sequence
    (:then_0
      ;[1 1 1] Try to cast to voxel procedural mesh component and complete SetBase() call
      (bind _asvoxel_procedural_mesh_component (Utilities|Casting|CastToVoxelProceduralMeshComponent NewBase))
      (bind _asvoxel_world (Utilities|Casting|CastToVoxelWorld (Components|GetOwner _asvoxel_procedural_mesh_component)))
      (LocalVariables|SetTheVoxelWorld _asvoxel_world))
    (:then_1
      ;[1 1 1] Try to handle instanced static mesh component
      (bind _asinstanced_static_mesh_component (Utilities|Casting|CastToInstancedStaticMeshComponent NewBase))
      (bind _asvoxel_world_2 (Utilities|Casting|CastToVoxelWorld (Components|GetOwner _asinstanced_static_mesh_component)))
      (LocalVariables|SetTheVoxelWorld _asvoxel_world_2))
    (:then_2
      ;[1 1 1] Otherwise return false and it will be handled in default way
      (return false)))
  ;[1 1 1] Try to complete SetBase call with voxel component info
  (bind _asprimitive_component (Utilities|Casting|CastToPrimitiveComponent (Variables|/Script/Engine.Actor|GetRootComponent (LocalVariables|GetTheVoxelWorld))))
  (Class|LocomotionCharacter|SetBaseNative _asprimitive_component BoneName bNotifyActor)
  (return true))