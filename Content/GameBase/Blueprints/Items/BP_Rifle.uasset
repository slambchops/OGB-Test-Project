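; Rifle item that fires a tracer round from its muzzle toward the player's aim point when used.
; UseItem calls SpawnProjectile, which reads the MuzzleSocket location and asks the owning LocomotionPlayer for its aiming location, ignoring the rifle.
; It then spawns BP_TracerRounds rotated from muzzle to aim point, with the rifle as Owner and the character as Instigator.
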(event EventBeginPlay)

(event Collision|EventActorBeginOverlap
  (params (OtherActor :type Actor%20Object%20Reference)))

(event EventTick
  (params (DeltaSeconds :type Float%20%28single-precision%29)))

(event EventUseItem
  (CallFunction|SpawnProjectile))

(fn ConstructionScript)

(fn SpawnProjectile
  (Utilities|FlowControl|Sequence
    (:then_0
      ;[1 1 1] Get variables need for line trace
      (LocalVariables|SetMuzzleLocation (Transformation|GetSocketLocation (Variables|Default|GetMeshComp) "MuzzleSocket")))
    (:then_1
      ;[1 1 1] Do line trace
      (bind _returnvalue (Class|OGBUsableItemComponent|GetOwningCharacter (Variables|Default|GetUseComp)))
      (bind _aslocomotion_player (Utilities|Casting|CastToLocomotionPlayer _returnvalue))
      (bind (_location _distance) (Class|LocomotionPlayer|GetAimingLocation _aslocomotion_player self false))
      (LocalVariables|SetHitLocation _location)
      (LocalVariables|SetDistance _distance)
      (LocalVariables|SetTracerTransform (Math|Transform|MakeTransform (LocalVariables|GetMuzzleLocation) (Math|Rotator|FindLookatRotation (LocalVariables|GetMuzzleLocation) (LocalVariables|GetHitLocation)))))
    (:then_2
      ;[1 1 1] Spawn tracer
      (bind _returnvalue_2 (Class|OGBUsableItemComponent|GetOwningCharacter (Variables|Default|GetUseComp)))
      (Game|SpawnActorfromClass "/OGB_Gameplay_Core/Blueprints/Projectiles/BP_TracerRounds.BP_TracerRounds_C" (LocalVariables|GetTracerTransform) "AdjustIfPossibleButAlwaysSpawn" self _returnvalue_2))))