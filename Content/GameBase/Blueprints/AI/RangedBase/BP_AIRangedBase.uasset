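; BP_AIRangedBase is a base Blueprint for ranged AI enemies, with mostly stubbed combat functions.
; Alive state comes from the OGBHealth component, and attack state from the IsAttacking variable.
; Target and focal-location functions defer to the parent, with target updates also cached in CurrentTarget.
; Montage, damage-effect and melee-attack functions return false or zero without acting, and BeginPlay and Tick are empty.
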(event EventBeginPlay)

(event Collision|EventActorBeginOverlap
  (params (OtherActor :type Actor%20Object%20Reference)))

(event EventTick
  (params (DeltaSeconds :type Float%20%28single-precision%29)))

(fn ConstructionScript)

(fn StartAnimMontage
  (params (TheMontage :type Anim%20Montage%20Object%20Reference))
  (return false))

(fn IsAttacking
  (return (Variables|Attack|GetbIsAttacking)))

(fn IsAlive
  (bind _returnvalue (Class|OGBHealthComponent|IsAlive (Variables|Default|GetOGBHealth)))
  (return _returnvalue))

(fn ApplyDamageEffect
  (params (HitResult :type Hit%20Result%20Structure))
  (return false))

(fn UpdateEnemyTarget
  (params (NewTarget :type Actor%20Object%20Reference))
  (bind _returnvalue (|CallParentFunction NewTarget))
  (Variables|Attack|SetCurrentTarget NewTarget)
  (return _returnvalue))

(fn StartMeleeAttack
  (return 0.0 false))

(fn SetFocalLocation
  (params (NewLocation :type Vector :default "0, 0, 0"))
  (bind _returnvalue (|CallParentFunction NewLocation))
  (return _returnvalue))

(fn ClearFocalLocation
  (bind _returnvalue (|CallParentFunction))
  (return _returnvalue))