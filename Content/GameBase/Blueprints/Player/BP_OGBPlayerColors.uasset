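; Player character Blueprint that gives each body-part material slot its own color, producing randomized outfits replicated over the network.
; Construction creates a dynamic material per slot, stores them in MatInstanceTable and paints all with SkinColor.
; InitColors, not called within this file, randomizes shirt, sleeves, pants and shoes on the server, while remote controlled instances request a sync.
; SyncColors reads colors back from the materials and multicasts them by table index.
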(event Custom|ServerUpdateColors
  (ColoringSystem|SyncColors))

(event Custom|MulticastUpdateColor
  (params (Colors :type Array%20of%20Linear%20Color%20Structures))
  (for (_array_element _array_index) (Variables|ColoringSystem|GetMatInstanceTable)
    (Rendering|Material|SetVectorParameterValue _array_element "BaseColor" (Utilities|Array|Get(acopy) Colors _array_index) :!class /Script/Engine.MaterialInstanceDynamic)))

(event EventBeginPlay
  (|CallParentFunction))

(event Collision|EventActorBeginOverlap
  (params (OtherActor :type Actor%20Object%20Reference))
  (|CallParentFunction OtherActor) ; This node is disabled and will not be called.\nDrag off pins to build functionality.
)

(event EventTick
  (params (DeltaSeconds :type Float%20%28single-precision%29))
  (|CallParentFunction DeltaSeconds) ; This node is disabled and will not be called.\nDrag off pins to build functionality.
)

(fn ConstructionScript
  (|CallParentFunction)
  (ColoringSystem|SetDynamicMaterials)
  (ColoringSystem|SetDefaultColors))

(fn SetDynamicMaterials
  (Utilities|FlowControl|Sequence
    (:then_0
      (bind _returnvalue (Rendering|Material|CreateDynamicMaterialInstance (Variables|Character|GetMesh) 2 0 "None" :!class /Script/Engine.PrimitiveComponent))
      (bind _output_get (Variables|ColoringSystem|SetHead _returnvalue))
      (Utilities|Array|Add (Variables|ColoringSystem|GetMatInstanceTable) _output_get)
      (bind _returnvalue_2 (Rendering|Material|CreateDynamicMaterialInstance (Variables|Character|GetMesh) 1 0 "None" :!class /Script/Engine.PrimitiveComponent))
      (bind _output_get_2 (Variables|ColoringSystem|SetTorso _returnvalue_2))
      (Utilities|Array|Add (Variables|ColoringSystem|GetMatInstanceTable) _output_get_2)
      (bind _returnvalue_3 (Rendering|Material|CreateDynamicMaterialInstance (Variables|Character|GetMesh) 0 0 "None" :!class /Script/Engine.PrimitiveComponent))
      (bind _output_get_3 (Variables|ColoringSystem|SetPelvis _returnvalue_3))
      (Utilities|Array|Add (Variables|ColoringSystem|GetMatInstanceTable) _output_get_3))
    (:then_1
      (bind _returnvalue_4 (Rendering|Material|CreateDynamicMaterialInstance (Variables|Character|GetMesh) 6 0 "None" :!class /Script/Engine.PrimitiveComponent))
      (bind _output_get_4 (Variables|ColoringSystem|SetUpperLegs _returnvalue_4))
      (Utilities|Array|Add (Variables|ColoringSystem|GetMatInstanceTable) _output_get_4)
      (bind _returnvalue_5 (Rendering|Material|CreateDynamicMaterialInstance (Variables|Character|GetMesh) 7 0 "None" :!class /Script/Engine.PrimitiveComponent))
      (bind _output_get_5 (Variables|ColoringSystem|SetLowerLegs _returnvalue_5))
      (Utilities|Array|Add (Variables|ColoringSystem|GetMatInstanceTable) _output_get_5)
      (bind _returnvalue_6 (Rendering|Material|CreateDynamicMaterialInstance (Variables|Character|GetMesh) 8 0 "None" :!class /Script/Engine.PrimitiveComponent))
      (bind _output_get_6 (Variables|ColoringSystem|SetFeet _returnvalue_6))
      (Utilities|Array|Add (Variables|ColoringSystem|GetMatInstanceTable) _output_get_6))
    (:then_2
      (bind _returnvalue_7 (Rendering|Material|CreateDynamicMaterialInstance (Variables|Character|GetMesh) 4 0 "None" :!class /Script/Engine.PrimitiveComponent))
      (bind _output_get_7 (Variables|ColoringSystem|SetShoulder_L _returnvalue_7))
      (Utilities|Array|Add (Variables|ColoringSystem|GetMatInstanceTable) _output_get_7)
      (bind _returnvalue_8 (Rendering|Material|CreateDynamicMaterialInstance (Variables|Character|GetMesh) 3 0 "None" :!class /Script/Engine.PrimitiveComponent))
      (bind _output_get_8 (Variables|ColoringSystem|SetUpperArm_L _returnvalue_8))
      (Utilities|Array|Add (Variables|ColoringSystem|GetMatInstanceTable) _output_get_8)
      (bind _returnvalue_9 (Rendering|Material|CreateDynamicMaterialInstance (Variables|Character|GetMesh) 5 0 "None" :!class /Script/Engine.PrimitiveComponent))
      (bind _output_get_9 (Variables|ColoringSystem|SetLowerArm_L _returnvalue_9))
      (Utilities|Array|Add (Variables|ColoringSystem|GetMatInstanceTable) _output_get_9)
      (bind _returnvalue_10 (Rendering|Material|CreateDynamicMaterialInstance (Variables|Character|GetMesh) 9 0 "None" :!class /Script/Engine.PrimitiveComponent))
      (bind _output_get_10 (Variables|ColoringSystem|SetHand_L _returnvalue_10))
      (Utilities|Array|Add (Variables|ColoringSystem|GetMatInstanceTable) _output_get_10))
    (:then_3
      (bind _returnvalue_11 (Rendering|Material|CreateDynamicMaterialInstance (Variables|Character|GetMesh) 12 0 "None" :!class /Script/Engine.PrimitiveComponent))
      (bind _output_get_11 (Variables|ColoringSystem|SetShoulder_R _returnvalue_11))
      (Utilities|Array|Add (Variables|ColoringSystem|GetMatInstanceTable) _output_get_11)
      (bind _returnvalue_12 (Rendering|Material|CreateDynamicMaterialInstance (Variables|Character|GetMesh) 11 0 "None" :!class /Script/Engine.PrimitiveComponent))
      (bind _output_get_12 (Variables|ColoringSystem|SetUpperArm_R _returnvalue_12))
      (Utilities|Array|Add (Variables|ColoringSystem|GetMatInstanceTable) _output_get_12)
      (bind _returnvalue_13 (Rendering|Material|CreateDynamicMaterialInstance (Variables|Character|GetMesh) 13 0 "None" :!class /Script/Engine.PrimitiveComponent))
      (bind _output_get_13 (Variables|ColoringSystem|SetLowerArm_R _returnvalue_13))
      (Utilities|Array|Add (Variables|ColoringSystem|GetMatInstanceTable) _output_get_13)
      (bind _returnvalue_14 (Rendering|Material|CreateDynamicMaterialInstance (Variables|Character|GetMesh) 14 0 "None" :!class /Script/Engine.PrimitiveComponent))
      (bind _output_get_14 (Variables|ColoringSystem|SetHand_R _returnvalue_14))
      (Utilities|Array|Add (Variables|ColoringSystem|GetMatInstanceTable) _output_get_14))))

(fn SetDefaultColors
  ;[1 1 1] Skin color -- set whole body
  (Rendering|Material|SetVectorParameterValue (Variables|ColoringSystem|GetHead) "BaseColor" (Variables|ColoringSystem|GetSkinColor) :!class /Script/Engine.MaterialInstanceDynamic))

(fn InitColors
  (Networking|SwitchHasAuthority
    (:Authority
      (Utilities|FlowControl|Sequence
        (:then_0
          ;[1 1 1] Set shirt color
          (bind _output_get (LocalVariables|SetRandomColor ""))
          (Class|KismetMathLibrary|LinearColorSetRandomHue _output_get)
          (Rendering|Material|SetVectorParameterValue (Variables|ColoringSystem|GetTorso) "BaseColor" (LocalVariables|GetRandomColor) :!class /Script/Engine.MaterialInstanceDynamic)
          ;[1 1 1] Randomly decide if shirt has sleeves
          (if (Math|Random|RandomBool)
            (Rendering|Material|SetVectorParameterValue (Variables|ColoringSystem|GetUpperArm_R) "BaseColor" (LocalVariables|GetRandomColor) :!class /Script/Engine.MaterialInstanceDynamic)
            (if (Math|Random|RandomBool)
              (Rendering|Material|SetVectorParameterValue (Variables|ColoringSystem|GetLowerArm_L) "BaseColor" (LocalVariables|GetRandomColor) :!class /Script/Engine.MaterialInstanceDynamic))))
        (:then_1
          ;[1 1 1] Set pants color
          (bind _output_get_2 (LocalVariables|SetRandomColor ""))
          (Class|KismetMathLibrary|LinearColorSetRandomHue _output_get_2)
          (Rendering|Material|SetVectorParameterValue (Variables|ColoringSystem|GetPelvis) "BaseColor" (LocalVariables|GetRandomColor) :!class /Script/Engine.MaterialInstanceDynamic)
          ;[1 1 1] Randomly decide if pants or shorts
          (if (Math|Random|RandomBool)
            (Rendering|Material|SetVectorParameterValue (Variables|ColoringSystem|GetLowerLegs) "BaseColor" (LocalVariables|GetRandomColor) :!class /Script/Engine.MaterialInstanceDynamic)))
        (:then_2
          ;[1 1 1] Set shoes color
          (bind _output_get_3 (LocalVariables|SetRandomColor ""))
          (Class|KismetMathLibrary|LinearColorSetRandomHue _output_get_3)
          (Rendering|Material|SetVectorParameterValue (Variables|ColoringSystem|GetFeet) "BaseColor" (LocalVariables|GetRandomColor) :!class /Script/Engine.MaterialInstanceDynamic))))
    (:Remote
      (Utilities|IsValid (Pawn|GetController)
        (:Is%20Valid
          (CallFunction|ServerUpdateColors))))))

(fn SyncColors
  (Networking|SwitchHasAuthority
    (:Authority
      (Utilities|FlowControl|Sequence
        (:then_0
          (for _array_element (Variables|ColoringSystem|GetMatInstanceTable)
            (bind _returnvalue (Rendering|Material|GetVectorParameterValue _array_element "BaseColor" :!class /Script/Engine.MaterialInstanceDynamic))
            (Utilities|Array|Add (LocalVariables|GetColorArray) _returnvalue)))
        (:then_1
          (CallFunction|MulticastUpdateColor (LocalVariables|GetColorArray)))))))