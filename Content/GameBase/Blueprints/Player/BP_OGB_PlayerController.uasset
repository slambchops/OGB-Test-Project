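; Player controller Blueprint for the OGB game base that ties the menu toggle to the pawn's vanity mode.
; ToggleMenu calls the parent implementation, then casts the controlled pawn to LocomotionPlayer and sets its VanityMode to the current menu-open state, returning that value.
; For other pawns it returns the parent result; BeginPlay and construction only call their parents.
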(event EventBeginPlay
  (|CallParentFunction))

(event EventTick
  (params (DeltaSeconds :type Float%20%28single-precision%29))
  (|CallParentFunction DeltaSeconds) ; This node is disabled and will not be called.\nDrag off pins to build functionality.
)

(fn ConstructionScript
  (|CallParentFunction))

(fn ToggleMenu
  (bind _returnvalue (|CallParentFunction))
  (bind _aslocomotion_player (Utilities|Casting|CastToLocomotionPlayer (Pawn|GetControlledPawn))
    (:then
      (bind _returnvalue_2 (Class|OGBPlayerController|IsMenuOpen))
      (bind _output_get (Variables|/Script/OGB_Loco.LocomotionPlayer|SetbVanityMode _aslocomotion_player _returnvalue_2))
      (return _output_get))
    (:CastFailed
      (return _returnvalue))))