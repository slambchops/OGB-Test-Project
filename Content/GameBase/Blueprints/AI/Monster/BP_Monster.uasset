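; AI monster character with server-authoritative melee combat, target-based movement speed and ragdoll death.
; Melee attacks multicast a random montage when the blackboard enemy is in range, and speed changes and death are also multicast.
; Anim events trigger hit checks that pick a hand socket or actor origin by gameplay tag or string, then apply damage by distance.
; Hand melee components attach to bones, but the overlap-check function is never called here.
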(event Custom|MulticastDeath
  (CallFunction|StartRagdoll)
  (Actor|SetLifeSpan 5.0)
  (Class|Pawn|DetachfromControllerPendingDestroy))

(event Custom|MulticastMontage
  (params (AttackMontage :type Anim%20Montage%20Object%20Reference))
  (Animation|Montage|PlayMontage (Variables|Character|GetMesh) AttackMontage))

(event Custom|MulticastUpdateMovementSpeed
  (params (NewMovementSpeed :type Float%20%28single-precision%29))
  (Variables|/Script/Engine.CharacterMovementComponent|SetMaxWalkSpeed (Variables|Character|GetCharacterMovement) NewMovementSpeed))

(event EventBeginPlay
  ;[1 1 1] Health component events
  (EventDispatchers|BindEventtoOnTakeDamage (Variables|Default|GetOGBHealth) (EventDispatchers|CreateEvent :!event OnTakeDamage)))

(event Collision|EventActorBeginOverlap
  (params (OtherActor :type Actor%20Object%20Reference)))

(event EventTick
  (params (DeltaSeconds :type Float%20%28single-precision%29)))

(event EventOnAnimEvent
  (params (Event :type Anim%20Event%20Structure))
  (CallFunction|HandleAnimEvent Event))

(fn ConstructionScript
  (Transformation|AttachComponentToComponent (Variables|Default|GetRightHandMeleeComp) (Variables|Character|GetMesh) (Variables|MeleeAttack|GetRightHandBone) "SnapToTarget" "SnapToTarget" "KeepRelative" true)
  (Transformation|AttachComponentToComponent (Variables|Default|GetLeftHandMeleeComp) (Variables|Character|GetMesh) (Variables|MeleeAttack|GetLeftHandBone) "SnapToTarget" "SnapToTarget" "KeepRelative" true))

(fn OnTakeDamage
  (params (HealthComp :type OGB%20Health%20Component%20Object%20Reference) (Health :type Float%20%28single-precision%29) (HealthDelta :type Float%20%28single-precision%29) (DamageType :type Damage%20Type%20Object%20Reference) (InstigatedBy :type Controller%20Object%20Reference) (DamageCauser :type Actor%20Object%20Reference))
  (Networking|SwitchHasAuthority
    (:Authority
      (if (and (<= Health 0.0) (not (Variables|Health|GetbDied)))
        (CallFunction|MulticastDeath)
        (Variables|Health|SetbDied true)))))

(fn StartRagdoll
  (bind _mesh (Variables|Character|GetMesh))
  (Utilities|FlowControl|Sequence
    (:then_1
      ;[1 1 1] Update collision
      (Collision|SetCollisionProfileName _mesh "\"Ragdoll\"" :!class /Script/Engine.PrimitiveComponent)
      (Collision|SetCollisionObjectType _mesh "ECC_PhysicsBody")
      (Collision|SetCollisionEnabled _mesh "QueryAndPhysics")
      (Variables|/Script/Engine.PrimitiveComponent|SetbReplicatePhysicsToAutonomousProxy _mesh false)
      (Class|SkeletalMeshComponent|SetAllBodiesBelowSimulatePhysics _mesh (LocalVariables|GetRagdollBone) true true))))

(fn HandleUpdateEnemyTarget
  (params (NewTarget :type Actor%20Object%20Reference))
  (Networking|SwitchHasAuthority
    (:Authority
      ;[1 1 1] Update movement speed based on whether a target is found
      (Utilities|IsValid NewTarget
        (:Is%20Valid
          (LocalVariables|SetNewSpeed (Variables|Movement|GetFastSpeed)))
        (:Is%20Not%20Valid
          (LocalVariables|SetNewSpeed (Variables|Movement|GetSlowSpeed))))
      (CallFunction|MulticastUpdateMovementSpeed (LocalVariables|GetNewSpeed)))))

(fn HandleStartMeleeAttack
  (bind _meleeattacks_light (Variables|MeleeAttack|GetMeleeAttacks_Light))
  (bind _meleeattacks_light_2 (Variables|MeleeAttack|GetMeleeAttacks_Light))
  (bind _returnvalue (Utilities|Array|Length _meleeattacks_light_2))
  (bind _returnvalue_2 (Math|Random|RandomInteger _returnvalue))
  (bind _output (Utilities|Array|Get(acopy) _meleeattacks_light _returnvalue_2))
  (Utilities|FlowControl|Sequence
    (:then_0
      (Networking|SwitchHasAuthority
        (:Authority
          (bind _asactor (Utilities|Casting|CastToActor (AI|Components|Blackboard|GetValueasObject (AI|GetBlackboard 0) (Variables|Blackboard|GetBB_EnemyKeyName))))
          (bind _output_get (LocalVariables|SetEnemyToAttack _asactor))
          (Utilities|IsValid _output_get
            (:Is%20Valid
              (if (<= (Math|Vector|Distance(Vector) (Transformation|GetActorLocation _asactor) (Transformation|GetActorLocation)) (Variables|MeleeAttack|GetInRangeForAttack))
                (CallFunction|MulticastMontage _output)
                (bind _returnvalue_3 (Animation|GetPlayLength _output))
                (return true _returnvalue_3)))))))
    (:then_1
      (return false 0.0))))

(fn MeleeHitCheck
  (params (Tag :type Gameplay%20Tag%20Structure) (StringTag :type String))
  ;[1 1 1] Only do hit check on server
  (Networking|SwitchHasAuthority
    (:Authority
      ;[1 1 1] Make sure there is a valid melee target
      (bind _asogbaicontroller_base (Utilities|Casting|CastToOGBAIControllerBase (Pawn|GetController)))
      (bind _output_get (LocalVariables|SetMeleeTarget (Variables|/Script/OGB_Gameplay_Core.OGBAIControllerBase|GetCurrentEnemyTarget _asogbaicontroller_base)))
      (Utilities|IsValid _output_get
        (:Is%20Valid
          (Utilities|FlowControl|Sequence
            (:then_0
              ;[1 1 1] Determine how the attack should be processed based on gameplay tags
              (|SwitchGameplayTag Tag
                (:Default
                  (if (Utilities|String|Contains StringTag "right")
                    (LocalVariables|SetbRightHandAttack true)
                    (elif (Utilities|String|Contains StringTag "left")
                      (LocalVariables|SetbRightHandAttack false)
                      (else
                        (LocalVariables|SetbDefaultAttack true)))))
                (:Attack.Melee.LeftHand
                  (LocalVariables|SetbRightHandAttack false))
                (:Attack.Melee.RightHand
                  (LocalVariables|SetbRightHandAttack true))))
            (:then_1
              (if (LocalVariables|GetbDefaultAttack)
                ;[1 1 1] Default attack (just use line trace from character position)
                (bind _bhit (Attack|MeleeHitDIstanceCheck (Transformation|GetActorLocation) (LocalVariables|GetMeleeTarget)))
                (LocalVariables|SetbHit _bhit)
                (elif (LocalVariables|GetbRightHandAttack)
                  ;[1 1 1] Right hand attack
                  (bind _bhit_2 (Attack|MeleeHitDIstanceCheck (Transformation|GetSocketLocation (Variables|Character|GetMesh) (Variables|MeleeAttack|GetRightHandBone)) (LocalVariables|GetMeleeTarget)))
                  (LocalVariables|SetbHit _bhit_2)
                  (else
                    ;[1 1 1] Left hand
                    (bind _bhit_3 (Attack|MeleeHitDIstanceCheck (Transformation|GetSocketLocation (Variables|Character|GetMesh) (Variables|MeleeAttack|GetLeftHandBone)) (LocalVariables|GetMeleeTarget)))
                    (LocalVariables|SetbHit _bhit_3)))))
            (:then_2
              ;[1 1 1] Process the hit
              (if (LocalVariables|GetbHit)
                (Game|Damage|ApplyDamage (LocalVariables|GetMeleeTarget) (Variables|MeleeAttack|GetMeleeDamage) (Pawn|GetController) self)))))))))

(fn HandleAnimEvent
  (params (Event :type Anim%20Event%20Structure))
  (bind (_animnotify _tag _stringtag) (Utilities|Struct|BreakAnimEvent Event))
  (LocalVariables|SetAnimNotify _animnotify)
  (LocalVariables|SetTag _tag)
  (LocalVariables|SetStringTag _stringtag)
  (switch Utilities|FlowControl|Switch|SwitchonELocoAnimNotify (LocalVariables|GetAnimNotify)
    (:MeleeAttack
      (Attack|MeleeHitCheck (LocalVariables|GetTag) (LocalVariables|GetStringTag)))))

(fn MeleeHitDIstanceCheck
  (params (Origin :type Vector) (MeleeTarget :type Actor%20Object%20Reference))
  (bind _returnvalue (Transformation|GetActorLocation MeleeTarget))
  (Utilities|FlowControl|Sequence
    (:then_0
      ;[1 1 1] Check distance to target
      (LocalVariables|SetDistance (Math|Vector|Distance(Vector) Origin _returnvalue))
      ;[1 1 1] Debug line
      (if (Variables|Default|GetbDebug)
        (Rendering|Debug|DrawDebugLine Origin _returnvalue "(R=0.000000,G=1.000000,B=0.000000,A=1.000000)" 1.0 1.0)))
    (:then_1
      ;[1 1 1] Determine if hit occured
      (if (<= (LocalVariables|GetDistance) (Variables|MeleeAttack|GetMaxDistanceForHit))
        (return true)
        (else
          (return false))))))

(fn MeleeHitCollisionComponent
  (params (SphereComp :type Sphere%20Component%20Object%20Reference) (MeleeTarget :type Actor%20Object%20Reference))
  (for _array_element (Collision|GetOverlappingActors SphereComp 0 :!class /Script/Engine.PrimitiveComponent)
    (if (== _array_element MeleeTarget)
      (return true)))
  (return false))

(fn StartMeleeAttack
  (bind (_success _duration) (Attack|HandleStartMeleeAttack))
  (return _duration _success))

(fn UpdateEnemyTarget
  (params (NewTarget :type Actor%20Object%20Reference))
  (Attack|HandleUpdateEnemyTarget NewTarget)
  (return true))