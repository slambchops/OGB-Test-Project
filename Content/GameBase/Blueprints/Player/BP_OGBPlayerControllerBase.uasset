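; Base player controller Blueprint that extends menu toggling for pawns derived from BP_OGBPlayerBase.
; ToggleMenu calls the parent, then sets the pawn's VanityMode from IsMenuOpen and switches its menu lights to match.
; When the menu closes it restores the pawn's rotation mode to LookingDirection.
; For other pawns it returns the parent's result; BeginPlay and construction only call their parents.
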(event EventBeginPlay
  (|CallParentFunction))

(event EventTick
  (params (DeltaSeconds :type Float%20%28single-precision%29))
  (|CallParentFunction DeltaSeconds) ; This node is disabled and will not be called.\nDrag off pins to build functionality.
)

(fn ConstructionScript
  (|CallParentFunction))

(fn ToggleMenu
  (bind _returnvalue (|CallParentFunction))
  (bind _asbp_ogbplayer_base (Utilities|Casting|CastToBP_OGBPlayerBase (Pawn|GetControlledPawn))
    (:then
      (LocalVariables|SetLocoPlayer _asbp_ogbplayer_base)
      (bind _returnvalue_2 (Class|OGBPlayerController|IsMenuOpen))
      (bind _output_get (Variables|/Script/OGB_Loco.LocomotionPlayer|SetbVanityMode (LocalVariables|GetLocoPlayer) _returnvalue_2))
      (Default|EnableMenuLights (LocalVariables|GetLocoPlayer) _output_get)
      (if _output_get
        _
        (else
          (Class|LocomotionCharacter|SetRotationMode (LocalVariables|GetLocoPlayer) "LookingDirection")))
      (return _output_get))
    (:CastFailed
      (return _returnvalue))))